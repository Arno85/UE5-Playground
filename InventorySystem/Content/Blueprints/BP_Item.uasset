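; BP_Item is a pickup actor that shows an on-screen widget while the third-person character is in range.
; It creates a hidden WBP_Item widget on BeginPlay and toggles its visibility as the character begins and ends overlap.
; PickUpItem returns the stored Item value and triggers DestroyItem, which destroys the actor after a short delay.
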(event `self.ReceiveBeginPlay`
  (bind _returnvalue (`|CreateWidget` "/Game/Blueprints/WBP_Item.WBP_Item_C" (`GameplayStatics.GetPlayerController` 0)))
  (bind _output_get (set `self.WBP_Item` _returnvalue))
  (`UserWidget.AddToViewport` _output_get 0)
  (`Widget.SetVisibility` _output_get "Hidden"))

(event `self.ReceiveActorBeginOverlap`
  (params (OtherActor :type "Actor Object Reference"))
  (cast `/Game/ThirdPerson/Blueprints/BP_ThirdPersonCharacter` OtherActor)
  (`Widget.SetVisibility` (`self.WBP_Item`) "Visible"))

(event `self.ReceiveActorEndOverlap`
  (params (OtherActor :type "Actor Object Reference"))
  (cast `/Game/ThirdPerson/Blueprints/BP_ThirdPersonCharacter` OtherActor)
  (`Widget.SetVisibility` (`self.WBP_Item`) "Hidden"))

(event `Destroy Item`
  (`KismetSystemLibrary.Delay` 0.1)
  (`self.K2_DestroyActor`))

(fn `PickUpItem`
  (returns (Item :type String))
  (`self.Destroy Item`)
  (return (`self.Item`)))

(fn `UserConstructionScript`)